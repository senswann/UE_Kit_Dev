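; BPC_ScoreSystem is a manager component that counts AI kills as score and ends the game when a target is reached.
; On BeginPlay it binds to AI death events from the game mode's BPC_AiSystem, incrementing the score on each death.
; InitScore sets the maximum, enabling the limit only when it is positive; reaching it calls EndGame on the game mode's BPC_SceneManager.
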(event Custom|IADeath
  ;[1 1 1] Bind increase score on death IA event
  (CallFunction|IncreaseScore))

(event EventBeginPlay
  ;[1 1 1] Bind increase score on death IA event
  (EventDispatchers|BindEventtoIADeath (Actor|GetComponentbyClass (Game|GetGameMode) "/AiSystem/Blueprint/BPC_AiSystem.BPC_AiSystem_C") (delegate Custom|IADeath)))

(fn IncreaseScore
  ;[1 1 1] Increase Score
  (bind _result (Math|Integer|IncrementInt (Variables|Default|GetScore))
    (:%20%20
      (if (and (>= _result (Variables|Default|GetMaxScore)) (Variables|Default|GetSeeScore))
        ;[1 1 1] End game if Score >= MaxScore
        (Default|EndGame (Actor|GetComponentbyClass (Game|GetGameMode) "/SettingManager/SceneManager/Blueprint/BPC_SceneManager.BPC_SceneManager_C"))))))

(fn InitScore
  (params (Score :type Integer))
  ;[1 1 1] Init score
  (bind _output_get (Variables|Default|SetMaxScore Score))
  (Variables|Default|SetSeeScore (> _output_get 0)))