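; Shooter game mode that hosts the game's manager components: score, audio, graphics, save, scene/UI, object pool, AI and wave spawning.
; Its construction script reads the GameMode data table row to configure them, passing widget classes, pool actor class, max score and wave info.
; AI settings come from a separate IAGeneral row, and wave initialization runs only when that row is found.
; BeginPlay then initializes the pool.
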(event EventBeginPlay
  ;[1 1 1] Init at start of the game
  (Default|InitPool (Variables|Default|GetBPC_PoolSystem)))

(fn ConstructionScript
  (bind _bpc_audiomanager (Variables|Default|GetBPC_AudioManager))
  (bind _bpc_grapicsmanager (Variables|Default|GetBPC_GrapicsManager))
  (bind _bpc_savemanager (Variables|Default|GetBPC_SaveManager))
  (bind _bpc_scenemanager (Variables|Default|GetBPC_SceneManager))
  ;[0.4254 1 0.704] Init Widget
  (bind _returnvalue (Utilities|GetDataTableRow "/Game/GameRule/GameMode/DT_GameMode.DT_GameMode" "GameMode")
    (:then
      (Default|InitScore (Variables|Default|GetBPC_ScoreSystem) (.maxscore _returnvalue))
      ;;[1 1 1] Audio Setting Init
      (Variables|/SettingManager/AudioManager/Blueprint/BPC_AudioManager.BPC_AudioManager_C|SetWBPAudioSetting _bpc_audiomanager (Utilities|Struct|BreakSTR_AudioManager (.audiomanager _returnvalue)))
      (Default|InitAudioSetting _bpc_audiomanager)
      ;;[1 1 1] Graphic setting init
      (Variables|/SettingManager/GraphicManager/Blueprint/BPC_GrapicsManager.BPC_GrapicsManager_C|SetWBP_GraphicSetting _bpc_grapicsmanager (Utilities|Struct|BreakSTR_GraphicManager (.graphicmanager _returnvalue)))
      (Default|InitGraphicSetting _bpc_grapicsmanager)
      ;;[1 1 1] Save setting Init
      (Variables|/SettingManager/SaveManager/Blueprint/BPC_SaveManager.BPC_SaveManager_C|SetWBP_SaveSetting _bpc_savemanager (Utilities|Struct|BreakSTR_SaveSetting (.savemanager _returnvalue)))
      (Default|InitSaveSetting _bpc_savemanager)
      ;;[1 1 1] Scene manager Init
      (Variables|/SettingManager/SceneManager/Blueprint/BPC_SceneManager.BPC_SceneManager_C|SetWBPGameOverClass _bpc_scenemanager (.GameOverWidgetClass (Utilities|Struct|BreakSTR_SceneManager (.scenemanager _returnvalue))))
      (Variables|/SettingManager/SceneManager/Blueprint/BPC_SceneManager.BPC_SceneManager_C|SetWBPEndGameClass _bpc_scenemanager (.EndHGameWidgetClass (Utilities|Struct|BreakSTR_SceneManager (.scenemanager _returnvalue))))
      (Variables|/SettingManager/SceneManager/Blueprint/BPC_SceneManager.BPC_SceneManager_C|SetWBPPauseClass _bpc_scenemanager (.PauseWidgetClass (Utilities|Struct|BreakSTR_SceneManager (.scenemanager _returnvalue))))
      (Variables|/SettingManager/SceneManager/Blueprint/BPC_SceneManager.BPC_SceneManager_C|SetWBPSettingClass _bpc_scenemanager (.SettingWidgetClass (Utilities|Struct|BreakSTR_SceneManager (.scenemanager _returnvalue))))
      (Variables|/SettingManager/SceneManager/Blueprint/BPC_SceneManager.BPC_SceneManager_C|SetWBPHUDClass _bpc_scenemanager (.HUDWidgetClass (Utilities|Struct|BreakSTR_SceneManager (.scenemanager _returnvalue))))
      (Default|InitWidget _bpc_scenemanager)
      ;;[1 1 1] Init Pool system
      (Variables|/PoolSystem/Blueprint/BPC_PoolSystem.BPC_PoolSystem_C|SetActorClass (Variables|Default|GetBPC_PoolSystem) (Utilities|Struct|BreakSTR_PoolSystem (.poolsystem _returnvalue)))
      ;;[1 1 1] Init IA
      (bind _returnvalue_2 (Utilities|GetDataTableRow "/Game/GameRule/IA/DT_IAGeneral.DT_IAGeneral" "IAGeneral")
        (:then
          (Variables|/AiSystem/Blueprint/ManagerComponent/BPC_AiSystem.BPC_AiSystem_C|SetIA_General (Variables|Default|GetBPC_AiSystem) _returnvalue_2)
          ;;[1 1 1] Init Spawn Wave
          (Default|InitValue (Variables|Default|GetBPC_WaveSystem) (.WaveInfo (Utilities|Struct|BreakSTR_WaveSystem (.wavesystem _returnvalue))) (.MinRangePlayer (Utilities|Struct|BreakSTR_WaveSystem (.wavesystem _returnvalue)))))))))