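; Game mode for the main menu that displays the menu widget and switches the player to mouse-driven UI input.
; The construction script reads the menu widget class from the DT_GameMode data table, passes it to the BPCSceneManager component and initializes the menu there.
; BeginPlay adds that component's menu widget to the viewport, shows the cursor and sets UI-only input.
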(event EventBeginPlay
  (bind _returnvalue (Game|GetPlayerController 0))
  ;[1 1 1] Add widget to screen
  (UserInterface|Viewport|AddtoViewport (Variables|/SettingManager/SceneManager/Blueprint/BPC_SceneManager.BPC_SceneManager_C|GetMainMenu (Variables|Default|GetBPC_SceneManager)) 0)
  (Variables|/Script/Engine.PlayerController|SetbShowMouseCursor _returnvalue true)
  (Input|SetInputModeUIOnly _returnvalue 0 "DoNotLock" false))

(fn ConstructionScript
  (bind _bpc_scenemanager (Variables|Default|GetBPC_SceneManager))
  ;[1 1 1] Init main menu
  (bind _returnvalue (Utilities|GetDataTableRow "/Game/GameRule/GameMode/DT_GameMode.DT_GameMode" "GameMode")
    (:then
      (Variables|/SettingManager/SceneManager/Blueprint/BPC_SceneManager.BPC_SceneManager_C|SetWBPMainMenuClass _bpc_scenemanager (.MainMenuWidgetClass (Utilities|Struct|BreakSTR_SceneManager (.SceneManager (Utilities|Struct|BreakSTR_GameMode _returnvalue)))))
      (Default|InitMainMenu _bpc_scenemanager))))