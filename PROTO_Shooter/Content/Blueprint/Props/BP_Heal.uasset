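; BP_Heal is a pickup prop that heals the player on overlap.
; On BeginPlay it looks up its heal amount by NameID in the Heal map of the PropsInfo row in DT_PropsInfo.
; When the player character enters its box, it calls IncreaseHealth on the pawn's BPC_HealthSystem and destroys itself, but only if health is below maximum, so it stays in place otherwise.
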(event OnComponentBeginOverlap(Box)
  (params (OverlappedComponent :type Primitive%20Component%20Object%20Reference) (OtherActor :type Actor%20Object%20Reference) (OtherComp :type Primitive%20Component%20Object%20Reference) (OtherBodyIndex :type Integer) (bFromSweep :type Boolean) (SweepResult :type Hit%20Result%20Structure%20%28by%20ref%29))
  ;[1 1 1] If player overlap
  (if (== OtherActor (Game|GetPlayerCharacter 0))
    (CallFunction|Action)))

(event EventBeginPlay
  (CallFunction|InitValue))

(fn ConstructionScript)

(fn InitValue
  ;[1 1 1] Init value
  (bind _returnvalue (Utilities|GetDataTableRow "/Game/GameRule/Props/DT_PropsInfo.DT_PropsInfo" "PropsInfo")
    (:then
      (Variables|Default|SetHealToDeal (Utilities|Struct|BreakSTR_Heal (.Value (Utilities|Map|Find (Utilities|Struct|BreakSTR_PropsInfo _returnvalue) (Variables|Default|GetNameID))))))))

(fn Action
  (bind _returnvalue (Game|Player|GetPlayerPawn 0))
  (bind _returnvalue_2 (Actor|GetComponentbyClass _returnvalue "/HealthSystem/Blueprint/BPC_HealthSystem.BPC_HealthSystem_C"))
  ;[1 1 1] Heal player
  (if (< (Variables|/HealthSystem/Blueprint/BPC_HealthSystem.BPC_HealthSystem_C|GetCurrentHealth _returnvalue_2) (Variables|/HealthSystem/Blueprint/BPC_HealthSystem.BPC_HealthSystem_C|GetMaxHealth _returnvalue_2))
    (Default|IncreaseHealth _returnvalue_2 (Variables|Default|GetHealToDeal))
    (Actor|DestroyActor)))