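; BPC_DashSystem is a player component that dashes its owning Character along its current movement.
; The Dash event calls LaunchCharacter with the owner's velocity scaled by Power on all axes.
; Each call increments a counter, and a launch proceeds if no dash is active or the counter is within its limit.
; After DelayDash, it clears the dashing flag and decrements the counter if positive.
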(event Custom|Dash
  (params (Power :type Float%20%28double-precision%29) (DelayDash :type Float%20%28double-precision%29))
  (bind _returnvalue (Components|GetOwner))
  (bind _nb_dash (Variables|Default|GetNB_Dash))
  (bind _returnvalue_2 (Transformation|GetVelocity _returnvalue))
  (bind _returnvalue_3 (* _returnvalue_2 Power))
  ;[0.5636 0.1006 1] Dash Event
  (Math|Integer|IncrementInt (Variables|Default|GetNB_Dash)
    (:%20%20
      (if (or (not (Variables|Default|GetIsDashing)) (<= (Variables|Default|GetNB_Dash) (Variables|Default|GetNB_Dash_Limit)))
        (Variables|Default|SetIsDashing true)
        ;;[1 1 1] Launch player on the current direction
        (Character|LaunchCharacter (.AsCharacter (Utilities|Casting|CastToCharacter _returnvalue)) (Math|Vector|MakeVector (.x _returnvalue_3) (.y _returnvalue_3) (.z _returnvalue_3)) false false)
        (Utilities|FlowControl|Delay DelayDash)
        ;;[1 1 1] Reset value after delay
        (Variables|Default|SetIsDashing false)
        (if (> _nb_dash 0)
          (Math|Integer|DecrementInt _nb_dash))))))