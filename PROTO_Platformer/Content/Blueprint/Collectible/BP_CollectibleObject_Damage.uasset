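; Damage collectible that makes the player lose health when its interact action runs, noted as happening on overlap.
; The construction script looks up NameID in the DamageCollectible map of OtherElementStat to set DamageToDeal.
; The InterractAction override calls the parent, then passes that damage to DecreaseHealth on the BPCHealthSystem of player 0's BP_ThirdPersonCharacter.
; Its event graph holds only disabled default events, leaving triggering to the parent class.
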(event EventBeginPlay
  (|CallParentFunction) ; This node is disabled and will not be called.\nDrag off pins to build functionality.
)

(event Collision|EventActorBeginOverlap
  (params (OtherActor :type Actor%20Object%20Reference))
  (|CallParentFunction OtherActor) ; This node is disabled and will not be called.\nDrag off pins to build functionality.
)

(event EventTick
  (params (DeltaSeconds :type Float%20%28single-precision%29))
  (|CallParentFunction DeltaSeconds) ; This node is disabled and will not be called.\nDrag off pins to build functionality.
)

(fn ConstructionScript
  (bind _otherelementstat (Variables|Default|GetOtherElementStat))
  (bind _nameid (Variables|Default|GetNameID))
  (bind _damagecollectible (Utilities|Struct|BreakSTR_OtherElement _otherelementstat))
  (bind (_value _returnvalue) (Utilities|Map|Find _damagecollectible _nameid))
  (|CallParentFunction)
  ;[1 1 1] Set damage to deal
  (if _returnvalue
    (Variables|Default|SetDamageToDeal (.damagetodeal _value))))

(fn InterractAction
  ;[1 1 1] Loose HP when overlap object
  (|CallParentFunction)
  (bind _asbp_third_person_character (Utilities|Casting|CastToBP_ThirdPersonCharacter (Game|GetPlayerCharacter 0)))
  (Default|DecreaseHealth (Variables|/Game/Blueprint/BP_ThirdPersonCharacter.BP_ThirdPersonCharacter_C|GetBPC_HealthSystem _asbp_third_person_character) (Variables|Default|GetDamageToDeal)))