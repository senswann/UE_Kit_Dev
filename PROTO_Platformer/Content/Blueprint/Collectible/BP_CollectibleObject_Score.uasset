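; Score collectible for a platformer that adds points to the player's score when picked up.
; It overrides InterractAction, calling the parent, then adding ScoreToAdd through the BPCScoreSystem component on GM_Platformer and destroying itself.
; If the game mode is not GM_Platformer, it stops before scoring or destruction; the event graph holds only disabled default events.
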(event EventBeginPlay
  (|CallParentFunction) ; This node is disabled and will not be called.\nDrag off pins to build functionality.
)

(event Collision|EventActorBeginOverlap
  (params (OtherActor :type Actor%20Object%20Reference))
  (|CallParentFunction OtherActor) ; This node is disabled and will not be called.\nDrag off pins to build functionality.
)

(event EventTick
  (params (DeltaSeconds :type Float%20%28single-precision%29))
  (|CallParentFunction DeltaSeconds) ; This node is disabled and will not be called.\nDrag off pins to build functionality.
)

(fn ConstructionScript
  (|CallParentFunction))

(fn InterractAction
  ;[1 1 1] When Overlap add score point and destroy collectible
  (|CallParentFunction)
  (bind _asgm_platformer (Utilities|Casting|CastToGM_Platformer (Game|GetGameMode)))
  (Default|AddScore (Variables|/Game/Blueprint/Manager/GM_Platformer.GM_Platformer_C|GetBPC_ScoreSystem _asgm_platformer) (Variables|Default|GetScoreToAdd))
  (Actor|DestroyActor))