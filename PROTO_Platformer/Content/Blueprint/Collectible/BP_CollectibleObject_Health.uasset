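; Health pickup collectible that heals the player when collected.
; Overrides the parent collectible's InterractAction to call the parent, cast player 0 to BP_ThirdPersonCharacter and pass HealValue to IncreaseHealth on its BPCHealthSystem component.
; It then destroys itself, while its own event graph holds only disabled default events.
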(event EventBeginPlay
  (|CallParentFunction) ; This node is disabled and will not be called.\nDrag off pins to build functionality.
)

(event Collision|EventActorBeginOverlap
  (params (OtherActor :type Actor%20Object%20Reference))
  (|CallParentFunction OtherActor) ; This node is disabled and will not be called.\nDrag off pins to build functionality.
)

(event EventTick
  (params (DeltaSeconds :type Float%20%28single-precision%29))
  (|CallParentFunction DeltaSeconds) ; This node is disabled and will not be called.\nDrag off pins to build functionality.
)

(fn ConstructionScript
  (|CallParentFunction))

(fn InterractAction
  ;[1 1 1] Heal player when overlap object
  (|CallParentFunction)
  (bind _asbp_third_person_character (Utilities|Casting|CastToBP_ThirdPersonCharacter (Game|GetPlayerCharacter 0)))
  (Default|IncreaseHealth (Variables|/Game/Blueprint/BP_ThirdPersonCharacter.BP_ThirdPersonCharacter_C|GetBPC_HealthSystem _asbp_third_person_character) (Variables|Default|GetHealValue))
  (Actor|DestroyActor))