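; Base AI character that damages the player's health system when its capsule overlaps the third-person character.
; On BeginPlay, it converts its list of possible positions from actor-relative to world space by transforming each through the actor transform.
; After a brief delay, it calls NeedMove on its BP_AiController so it starts moving by default.
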(event OnComponentBeginOverlap(CapsuleComponent)
  (params (OverlappedComponent :type Primitive%20Component%20Object%20Reference) (OtherActor :type Actor%20Object%20Reference) (OtherComp :type Primitive%20Component%20Object%20Reference) (OtherBodyIndex :type Integer) (bFromSweep :type Boolean) (SweepResult :type Hit%20Result%20Structure%20%28by%20ref%29))
  ;[1 1 1] Take damage if player overlap
  (bind _asbp_third_person_character (Utilities|Casting|CastToBP_ThirdPersonCharacter OtherActor))
  (Default|DecreaseHealth (Variables|/Game/Blueprint/BP_ThirdPersonCharacter.BP_ThirdPersonCharacter_C|GetBPC_HealthSystem _asbp_third_person_character) (Variables|Default|GetDamageToDeal)))

(event EventBeginPlay
  (CallFunction|ReplacePosition)
  ;[1 1 1] Need Move by default
  (Utilities|FlowControl|Delay 0.01)
  (bind _asbp_ai_controller (Utilities|Casting|CastToBP_AiController (Pawn|GetController)))
  (Default|NeedMove _asbp_ai_controller))

(fn ConstructionScript
  (|CallParentFunction))

(fn ReplacePosition
  ;[1 1 1] replace vector by world location
  (for _array_element (Variables|Default|GetListOfPossiblePosition)
    (Utilities|Array|Add (LocalVariables|GetTMP_List) (Math|Transform|TransformLocation (Transformation|GetActorTransform) _array_element)))
  (Variables|Default|SetListOfPossiblePosition (LocalVariables|GetTMP_List)))