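; GM_Platformer is a platformer manager Blueprint that runs a play timer and configures the end-of-game and pause screens.
; A looping 0.05-second timer adds the current frame's world delta, not the elapsed interval, to Timer unless StopTimer is set, then updates WBPTimer if valid.
; The construction script passes the Game Over, End Game and Pause widget classes to BPCSceneManager.
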(event Custom|TimerEvent
  ;[1 1 1] Timer Logic
  (if (not (Variables|Default|GetStopTimer))
    (bind _output_get (Variables|Default|SetTimer (+ (Variables|Default|GetTimer) (Utilities|Time|GetWorldDeltaSeconds))))
    (bind _wbptimer (Variables|Default|GetWBPTimer)
      (:then
        (Default|UpdateTimer _wbptimer _output_get))
      (:else))))

(event EventBeginPlay
  ;[1 1 1] Timer Logic
  (Utilities|Time|SetTimerbyEvent (delegate Custom|TimerEvent) 0.05 true))

(fn ConstructionScript
  (bind _bpc_scenemanager (Variables|Default|GetBPC_SceneManager))
  ;[1 1 1] Set Game Over and End Game widget class & Pause UI
  (Variables|/SceneManager/Blueprint/BPC_SceneManager.BPC_SceneManager_C|SetWBPGameOverClass _bpc_scenemanager (Variables|Default|GetGameOverClass))
  (Variables|/SceneManager/Blueprint/BPC_SceneManager.BPC_SceneManager_C|SetWBPEndGameClass _bpc_scenemanager (Variables|Default|GetEndGameClass))
  (Variables|/SceneManager/Blueprint/BPC_SceneManager.BPC_SceneManager_C|SetWBPPauseClass _bpc_scenemanager (Variables|Default|GetPauseClass)))