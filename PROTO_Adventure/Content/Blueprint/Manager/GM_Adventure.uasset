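; Adventure game mode that hosts and configures the audio, graphics, save, scene and AI manager components.
; Its construction script reads widget classes from a DT_GameMode row into the audio, graphics, save and scene managers, then calls their init functions.
; It then feeds the general AI row from DT_IASystem to the AI system component.
; On BeginPlay it caches all BP_Props actors and adds the scene manager's HUD to the viewport.
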(event EventBeginPlay
  ;[1 1 1] Get all props
  (bind _outactors (Actor|GetAllActorsOfClass "/Game/Blueprint/Props/BP_Props.BP_Props_C"))
  (Variables|Default|SetPropsArray _outactors)
  ;[1 1 1] Load widget on begin
  (UserInterface|Viewport|AddtoViewport (Variables|/SettingManager/SceneManager/Blueprint/BPC_SceneManager.BPC_SceneManager_C|GetHUDWidget (Variables|Default|GetBPC_SceneManager)) 0))

(fn ConstructionScript
  (bind _bpc_audiomanager (Variables|Default|GetBPC_AudioManager))
  (bind _bpc_grapicsmanager (Variables|Default|GetBPC_GrapicsManager))
  (bind _bpc_savemanager (Variables|Default|GetBPC_SaveManager))
  (bind _bpc_scenemanager (Variables|Default|GetBPC_SceneManager))
  ;[0.2704 0.9768 1] Init Game Mode
  (bind _returnvalue (Utilities|GetDataTableRow "/Game/GameRule/GameMode/DT_GameMode.DT_GameMode" "GameMode")
    (:then
      ;;[1 1 1] Init Audio
      (Variables|/SettingManager/AudioManager/Blueprint/BPC_AudioManager.BPC_AudioManager_C|SetWBPAudioSetting _bpc_audiomanager (.audiowidgetclass (.AudioManager (Utilities|Struct|BreakSTR_GameMode _returnvalue))))
      (Default|InitAudioSetting _bpc_audiomanager)
      ;;[1 1 1] Init Graphic
      (Variables|/SettingManager/GraphicManager/Blueprint/BPC_GrapicsManager.BPC_GrapicsManager_C|SetWBP_GraphicSetting _bpc_grapicsmanager (.graphic_widget_class (.GraphicManager (Utilities|Struct|BreakSTR_GameMode _returnvalue))))
      (Default|InitGraphicSetting _bpc_grapicsmanager)
      ;;[1 1 1] Init Save
      (Variables|/SettingManager/SaveManager/Blueprint/BPC_SaveManager.BPC_SaveManager_C|SetWBP_SaveSetting _bpc_savemanager (.save_widget_class (.SaveManager (Utilities|Struct|BreakSTR_GameMode _returnvalue))))
      (Default|InitSaveSetting _bpc_savemanager)
      ;;[1 1 1] Init Scene manager
      (Variables|/SettingManager/SceneManager/Blueprint/BPC_SceneManager.BPC_SceneManager_C|SetWBPGameOverClass _bpc_scenemanager (.GameOverWidgetClass (Utilities|Struct|BreakSTR_SceneManager (.SceneManager (Utilities|Struct|BreakSTR_GameMode _returnvalue)))))
      (Variables|/SettingManager/SceneManager/Blueprint/BPC_SceneManager.BPC_SceneManager_C|SetWBPEndGameClass _bpc_scenemanager (.EndGameWidgetClass (Utilities|Struct|BreakSTR_SceneManager (.SceneManager (Utilities|Struct|BreakSTR_GameMode _returnvalue)))))
      (Variables|/SettingManager/SceneManager/Blueprint/BPC_SceneManager.BPC_SceneManager_C|SetWBPPauseClass _bpc_scenemanager (.PauseWidgetClass (Utilities|Struct|BreakSTR_SceneManager (.SceneManager (Utilities|Struct|BreakSTR_GameMode _returnvalue)))))
      (Variables|/SettingManager/SceneManager/Blueprint/BPC_SceneManager.BPC_SceneManager_C|SetWBPSettingClass _bpc_scenemanager (.SettingWidgetClass (Utilities|Struct|BreakSTR_SceneManager (.SceneManager (Utilities|Struct|BreakSTR_GameMode _returnvalue)))))
      (Variables|/SettingManager/SceneManager/Blueprint/BPC_SceneManager.BPC_SceneManager_C|SetWBPHUDClass _bpc_scenemanager (.HUDWidgetClass (Utilities|Struct|BreakSTR_SceneManager (.SceneManager (Utilities|Struct|BreakSTR_GameMode _returnvalue)))))
      (Default|InitWidget _bpc_scenemanager)
      ;;[1 1 1] Init IA
      (bind _returnvalue_2 (Utilities|GetDataTableRow "/Game/GameRule/IA/DT_IASystem.DT_IASystem" "IAGeneral")
        (:then
          (Variables|/AiSystem/Blueprint/ManagerComponent/BPC_AiSystem.BPC_AiSystem_C|SetIA_General (Variables|Default|GetBPC_AiSystem) _returnvalue_2))))))