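; BP_DialogZone is a trigger volume that plays a multi-camera dialog when the player interacts inside it or, with AutoTrigger, on entry.
; The construction script loads lines, speakers and camera indices from a DT_DialogSystem row.
; Overlap sets the player's DialogRef and HUD prompt, while Interact switches the view and input context.
; DialogLogic steps through lines, updating camera and widget, then restores default input and optionally disables the box for one-time dialogs.
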(event OnComponentBeginOverlap(Box)
  (params (OverlappedComponent :type Primitive%20Component%20Object%20Reference) (OtherActor :type Actor%20Object%20Reference) (OtherComp :type Primitive%20Component%20Object%20Reference) (OtherBodyIndex :type Integer) (bFromSweep :type Boolean) (SweepResult :type Hit%20Result%20Structure%20%28by%20ref%29))
  ;[1 1 1] Set dialog ref of the player
  (bind _asbp_third_person_character (Utilities|Casting|CastToBP_ThirdPersonCharacter OtherActor))
  (Variables|/Game/Blueprint/Character/BP_ThirdPersonCharacter.BP_ThirdPersonCharacter_C|SetDialogRef _asbp_third_person_character self)
  (Default|InteractPreview (Variables|/SettingManager/SceneManager/Blueprint/BPC_SceneManager.BPC_SceneManager_C|GetHUDWidget (Actor|GetComponentbyClass (Game|GetGameMode) "/SettingManager/SceneManager/Blueprint/BPC_SceneManager.BPC_SceneManager_C")) true)
  (if (Variables|Check|GetAutoTrigger?)
    (CallFunction|Interact)))

(event OnComponentEndOverlap(Box)
  (params (OverlappedComponent :type Primitive%20Component%20Object%20Reference) (OtherActor :type Actor%20Object%20Reference) (OtherComp :type Primitive%20Component%20Object%20Reference) (OtherBodyIndex :type Integer))
  ;[1 1 1] Loose ref of the dialog
  (bind _asbp_third_person_character (Utilities|Casting|CastToBP_ThirdPersonCharacter OtherActor))
  (Variables|/Game/Blueprint/Character/BP_ThirdPersonCharacter.BP_ThirdPersonCharacter_C|SetDialogRef _asbp_third_person_character 0)
  (Default|InteractPreview (Variables|/SettingManager/SceneManager/Blueprint/BPC_SceneManager.BPC_SceneManager_C|GetHUDWidget (Actor|GetComponentbyClass (Game|GetGameMode) "/SettingManager/SceneManager/Blueprint/BPC_SceneManager.BPC_SceneManager_C")) false))

(event EventBeginPlay
  ;[1 1 1] get all camera of the actor
  (CallFunction|InitCameraArray)
  (CallFunction|ActiveCamera))

(fn ConstructionScript
  (bind _dialog (Variables|Dialog|GetDialog))
  ;[1 1 1] Init dialog daata
  (bind _returnvalue (Utilities|GetDataTableRow "/Game/GameRule/Dialog/DT_DialogSystem.DT_DialogSystem" (Variables|Default|GetDialogRef))
    (:then
      (for _array_element (Utilities|Struct|BreakSTR_DialogSystem _returnvalue)
        (Utilities|Array|Add _dialog (.Dialog (Utilities|Struct|BreakSTR_Dialog _array_element)))
        (Utilities|Array|Add (Variables|Dialog|GetWhoTalk) (.WhoTalk (Utilities|Struct|BreakSTR_Dialog _array_element)))
        (Utilities|Array|Add (Variables|Dialog|GetCameraIndex) (.CameraIndex (Utilities|Struct|BreakSTR_Dialog _array_element))))
      (Variables|Default|SetDialogLength (Utilities|Array|Length _dialog)))))

(fn Interact
  ;[1 1 1] Interact logic
  (bind _asbp_third_person_character (Utilities|Casting|CastToBP_ThirdPersonCharacter (Game|Player|GetPlayerPawn 0)))
  (Default|SwitchCamera _asbp_third_person_character self "/Game/Input/IMC_Dialog.IMC_Dialog")
  (Default|Dialog (Variables|/SettingManager/SceneManager/Blueprint/BPC_SceneManager.BPC_SceneManager_C|GetHUDWidget (Actor|GetComponentbyClass (Game|GetGameMode) "/SettingManager/SceneManager/Blueprint/BPC_SceneManager.BPC_SceneManager_C")) true)
  (CallFunction|DialogLogic))

(fn DialogLogic
  (bind _returnvalue (Game|GetGameMode))
  (bind _returnvalue_2 (Actor|GetComponentbyClass _returnvalue "/SettingManager/SceneManager/Blueprint/BPC_SceneManager.BPC_SceneManager_C"))
  (bind _hudwidget (Variables|/SettingManager/SceneManager/Blueprint/BPC_SceneManager.BPC_SceneManager_C|GetHUDWidget _returnvalue_2))
  (bind _wbp_dialog (Variables|/SettingManager/SceneManager/Widget/WBP_HUD.WBP_HUD_C|GetWBP_Dialog _hudwidget))
  ;[0.7153 0.2178 1] Dialog logic
  (bind _result (Math|Integer|IncrementInt (Variables|Default|GetcurrentLength))
    (:%20%20
      (if (< _result (Variables|Default|GetDialogLength))
        ;;[1 1 1] IF we have next dialog
        (CallFunction|ActiveCamera (Utilities|Array|Get(acopy) (Variables|Dialog|GetCameraIndex) (Variables|Default|GetcurrentLength)))
        (Default|SetSpeeker _wbp_dialog (Utilities|Array|Get(acopy) (Variables|Dialog|GetWhoTalk) (Variables|Default|GetcurrentLength)))
        (Default|SetDialog _wbp_dialog (Utilities|Array|Get(acopy) (Variables|Dialog|GetDialog) (Variables|Default|GetcurrentLength)))
        (else
          ;;[1 1 1] If dialog end
          (Variables|Default|SetcurrentLength -1)
          (bind _asbp_third_person_character (Utilities|Casting|CastToBP_ThirdPersonCharacter (Game|Player|GetPlayerPawn 0)))
          (Variables|/Game/Blueprint/Character/BP_ThirdPersonCharacter.BP_ThirdPersonCharacter_C|SetDialogRef _asbp_third_person_character 0)
          (Default|SwitchCamera _asbp_third_person_character 0 "/Game/Input/IMC_Default.IMC_Default")
          (Default|Dialog _hudwidget false)
          (if (Variables|Check|GetOnceDialog?)
            (Collision|SetCollisionEnabled (Variables|Default|GetBox) "NoCollision")))))))

(fn ActiveCamera
  (params (CameraIndex :type Integer))
  ;[1 1 1] ActiveCameraLogic
  (for _array_element (Variables|Dialog|GetCameraArray)
    (Components|Activation|SetActive _array_element false false))
  (Components|Activation|SetActive (Utilities|Array|Get(acopy) (Variables|Dialog|GetCameraArray) CameraIndex) true false))

(fn InitCameraArray
  ;[1 1 1] Init camera array
  (bind _output_get (Variables|Dialog|SetCameraArray (Actor|GetComponentsByClass "/Script/Engine.CameraComponent")))
  (bind _output_get_2 (LocalVariables|SetNewLocalVar (Utilities|Array|Get(acopy) (Variables|Dialog|GetCameraArray) (Utilities|Array|LastIndex _output_get))))
  (Utilities|Array|RemoveIndex (Variables|Dialog|GetCameraArray) (Utilities|Array|LastIndex _output_get))
  (Utilities|Array|Insert (Variables|Dialog|GetCameraArray) _output_get_2))