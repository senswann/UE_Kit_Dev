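; Interactable transmission prop that plays a Level Sequence and activates or deactivates a linked PropsToActivate actor.
; Interact disables the box collision, then runs either a timed button (play, wait, reverse) or a toggle that plays or reverses based on IsReversePlay.
; When the sequence stops and re-interaction is allowed, it flips the direction and restores collision.
; BeginPlay creates the sequence player, and InitValue stops the point-of-interest component when POI is off.
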(event Custom|ButtonLogic
  ;[1 1 1] Button Logic
  (Sequencer|Player|Play (Variables|LevelSequence|GetLevelSequencePlayer) :!class /Script/MovieScene.MovieSceneSequencePlayer)
  (CallFunction|Action (Variables|Default|GetPropsToActivate))
  (Utilities|FlowControl|Delay (Variables|Default|GetDelayForButton))
  (Class|MovieSceneSequencePlayer|PlayReverse (Variables|LevelSequence|GetLevelSequencePlayer))
  (Default|SubAction (Variables|Default|GetPropsToActivate)))

(event Custom|EventStopSequence
  ;[1 1 1] Event when sequence end
  (if (Variables|Default|GetCanReiInterract?)
    (Variables|LevelSequence|SetIsReversePlay? (not (Variables|LevelSequence|GetIsReversePlay?)))
    (Collision|SetCollisionEnabled (Variables|Default|GetBox) "QueryAndPhysics")))

(event EventBeginPlay
  (CallFunction|InitValue)
  ;[1 1 1] Create Level Sequence player
  (bind _returnvalue (Sequencer|Player|CreateLevelSequencePlayer (Variables|LevelSequence|GetLevel%20Sequence)))
  (bind _output_get (Variables|LevelSequence|SetLevelSequencePlayer _returnvalue))
  (Utilities|IsValid _output_get
    (:Is%20Valid
      (EventDispatchers|BindEventtoOnStop _output_get (delegate Custom|EventStopSequence)))))

(fn ConstructionScript
  (|CallParentFunction))

(fn Interact
  ;[1 1 1] Activate actor
  (|CallParentFunction)
  (Collision|SetCollisionEnabled (Variables|Default|GetBox) "NoCollision")
  (if (> (Variables|Default|GetDelayForButton) 0.0)
    (CallFunction|ButtonLogic)
    (else
      (CallFunction|Action))))

(fn Action
  (bind _levelsequenceplayer (Variables|LevelSequence|GetLevelSequencePlayer))
  (bind _propstoactivate (Variables|Default|GetPropsToActivate))
  ;[1 1 1] activate props link
  (|CallParentFunction)
  (if (Variables|LevelSequence|GetIsReversePlay?)
    (Class|MovieSceneSequencePlayer|PlayReverse _levelsequenceplayer)
    (Default|SubAction _propstoactivate)
    (else
      (Sequencer|Player|Play _levelsequenceplayer :!class /Script/MovieScene.MovieSceneSequencePlayer)
      (CallFunction|Action _propstoactivate))))

(fn InitValue
  ;[1 1 1] Init Value
  (|CallParentFunction)
  (if (not (Variables|Default|GetPOI?))
    (Default|Stop (Variables|Default|GetBPC_PointOfInterest))))