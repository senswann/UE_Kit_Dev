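; BP_Props_Door is a door prop that opens on interaction when the player's inventory holds the required key.
; Interact either removes the key quantity from BPC_InventoryComponent if the key is consumable, or only checks that enough are held.
; On success, Action reports the door's objective ID to the player character, then opens the door by destroying the actor.
; Both functions extend parent implementations, and the event graph is unused.
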(event EventBeginPlay)

(event Collision|EventActorBeginOverlap
  (params (OtherActor :type Actor%20Object%20Reference)))

(event EventTick
  (params (DeltaSeconds :type Float%20%28single-precision%29)))

(fn ConstructionScript
  (|CallParentFunction))

(fn Interact
  (bind _returnvalue (Game|Player|GetPlayerPawn 0))
  (bind _keyidneed (Variables|Default|GetKeyIDNeed))
  (bind _keyquantity (Variables|Default|GetKeyQuantity))
  (bind _returnvalue_2 (Actor|GetComponentbyClass _returnvalue "/QuestSystem/Inventory/BPC_InventoryComponent.BPC_InventoryComponent_C"))
  ;[1 1 1] check if key need t oopen door
  (|CallParentFunction)
  (if (Variables|Default|GetIsKeyConsume)
    (bind _canremove_ (Default|RemovetoInvetory _returnvalue_2 _keyidneed _keyquantity))
    (if _canremove_
      (CallFunction|Action :!label _label))
    (else
      (bind _value (Default|QuerryInventory _returnvalue_2 _keyidneed))
      (if (>= _value _keyquantity)
        (goto _label)))))

(fn Action
  ;[1 1 1] Open door
  (|CallParentFunction)
  (Default|CallOnObjectiveIDCalled (CallFunction|GetMyPlayerCharacter) (Utilities|String|ToString(Name) (Variables|Default|GetObjectifID)) 1)
  (Actor|DestroyActor))