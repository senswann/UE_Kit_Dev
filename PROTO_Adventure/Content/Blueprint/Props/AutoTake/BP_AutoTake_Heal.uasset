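; Auto-take heal pickup prop that restores the player's health.
; It overrides the parent's Action function, calling the parent first, then reading the BPC_HealthSystem component on player pawn 0.
; If current health is below maximum, it increases health by HealToDeal and destroys itself; otherwise it stays in the world.
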(event EventBeginPlay
  (|CallParentFunction) ; This node is disabled and will not be called.\nDrag off pins to build functionality.
)

(event Collision|EventActorBeginOverlap
  (params (OtherActor :type Actor%20Object%20Reference))
  (|CallParentFunction OtherActor) ; This node is disabled and will not be called.\nDrag off pins to build functionality.
)

(event EventTick
  (params (DeltaSeconds :type Float%20%28single-precision%29))
  (|CallParentFunction DeltaSeconds) ; This node is disabled and will not be called.\nDrag off pins to build functionality.
)

(fn ConstructionScript
  (|CallParentFunction))

(fn Action
  (bind _returnvalue (Game|Player|GetPlayerPawn 0))
  (bind _returnvalue_2 (Actor|GetComponentbyClass _returnvalue "/HealthSystem/Blueprint/BPC_HealthSystem.BPC_HealthSystem_C"))
  ;[1 1 1] Get heal
  (|CallParentFunction)
  (if (< (Variables|/HealthSystem/Blueprint/BPC_HealthSystem.BPC_HealthSystem_C|GetCurrentHealth _returnvalue_2) (Variables|/HealthSystem/Blueprint/BPC_HealthSystem.BPC_HealthSystem_C|GetMaxHealth _returnvalue_2))
    (Default|IncreaseHealth _returnvalue_2 (Variables|Default|GetHealToDeal))
    (Actor|DestroyActor)))