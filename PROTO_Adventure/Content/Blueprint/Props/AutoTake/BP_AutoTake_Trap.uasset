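; BP_AutoTake_Trap is an auto-take prop that acts as a trap, damaging the player on overlap.
; Its Action override calls the parent, then DealDamage, which lowers player 0's health through the pawn's BPC_HealthSystem component.
; DealDamage disables the Box collision before the hit and restores it after a configurable delay, giving the trap a cooldown between hits.
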(event Custom|DealDamage
  ;[1 1 1] Deal damage
  (Collision|SetCollisionEnabled (Variables|Default|GetBox) "NoCollision")
  (Default|DecreaseHealth (Actor|GetComponentbyClass (Game|Player|GetPlayerPawn 0) "/HealthSystem/Blueprint/BPC_HealthSystem.BPC_HealthSystem_C") (Variables|Default|GetDamage))
  (Utilities|FlowControl|Delay (Variables|Default|GetDelay))
  (Collision|SetCollisionEnabled (Variables|Default|GetBox) "QueryAndPhysics"))

(event EventBeginPlay
  (|CallParentFunction) ; This node is disabled and will not be called.\nDrag off pins to build functionality.
)

(event Collision|EventActorBeginOverlap
  (params (OtherActor :type Actor%20Object%20Reference))
  (|CallParentFunction OtherActor) ; This node is disabled and will not be called.\nDrag off pins to build functionality.
)

(event EventTick
  (params (DeltaSeconds :type Float%20%28single-precision%29))
  (|CallParentFunction DeltaSeconds) ; This node is disabled and will not be called.\nDrag off pins to build functionality.
)

(fn ConstructionScript
  (|CallParentFunction))

(fn Action
  ;[1 1 1] when player overlap
  (|CallParentFunction)
  (CallFunction|DealDamage))