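; BP_Props_Pickup is an interactable prop that gives an item to the player's inventory when picked up.
; InitValue looks up NameID in the PropsPickup map of the DT_Props "Props" row to set the item ID and quantity.
; Interact runs the parent logic, passes those values to player 0's BPC_InventoryComponent through AddToInventory, then destroys the actor.
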(event EventBeginPlay
  (|CallParentFunction))

(event Collision|EventActorBeginOverlap
  (params (OtherActor :type Actor%20Object%20Reference)))

(event EventTick
  (params (DeltaSeconds :type Float%20%28single-precision%29)))

(fn ConstructionScript
  (|CallParentFunction))

(fn Interact
  ;[1 1 1] Interact add inventory
  (|CallParentFunction)
  (Default|AddtoInventory (Actor|GetComponentbyClass (Game|GetPlayerCharacter 0) "/QuestSystem/Inventory/BPC_InventoryComponent.BPC_InventoryComponent_C") (Variables|Default|GetObjectifID) (Variables|Default|GetQuantity))
  (Actor|DestroyActor))

(fn InitValue
  ;[1 1 1] Init Value
  (|CallParentFunction)
  (bind _returnvalue (Utilities|GetDataTableRow "/Game/GameRule/Other/Props/DT_Props.DT_Props" "Props")
    (:then
      (Variables|Default|SetQuantity (.Quantity (Utilities|Struct|BreakSTR_Props_Pickup (.Value (Utilities|Map|Find (.Props_Pickup (Utilities|Struct|BreakSTR_Props _returnvalue)) (Variables|Default|GetNameID))))))
      (Variables|Default|SetObjectifID (.ItemID (Utilities|Struct|BreakSTR_Props_Pickup (.Value (Utilities|Map|Find (.Props_Pickup (Utilities|Struct|BreakSTR_Props _returnvalue)) (Variables|Default|GetNameID)))))))))