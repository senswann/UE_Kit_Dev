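; BP_Props is a base interactable prop whose Box component defines the range in which the player can interact with it.
; On overlap it sets itself as BP_Character's PropsRef and shows the interact preview through BPC_SceneManager's HUD widget on the game mode, reversing both on exit.
; Interact, Action, SubAction and InitValue are empty hooks, apparently for child props to override, with InitValue called on BeginPlay.
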(event OnComponentBeginOverlap(Box)
  (params (OverlappedComponent :type Primitive%20Component%20Object%20Reference) (OtherActor :type Actor%20Object%20Reference) (OtherComp :type Primitive%20Component%20Object%20Reference) (OtherBodyIndex :type Integer) (bFromSweep :type Boolean) (SweepResult :type Hit%20Result%20Structure%20%28by%20ref%29))
  ;[1 1 1] Player overlap props range
  (bind _asbp_character (Utilities|Casting|CastToBP_Character OtherActor))
  (Variables|/Game/Blueprint/Character/BP_Character.BP_Character_C|SetPropsRef _asbp_character self)
  (Default|InteractPreview (Variables|/SettingManager/SceneManager/Blueprint/BPC_SceneManager.BPC_SceneManager_C|GetHUDWidget (Actor|GetComponentbyClass (Game|GetGameMode) "/SettingManager/SceneManager/Blueprint/BPC_SceneManager.BPC_SceneManager_C")) true))

(event OnComponentEndOverlap(Box)
  (params (OverlappedComponent :type Primitive%20Component%20Object%20Reference) (OtherActor :type Actor%20Object%20Reference) (OtherComp :type Primitive%20Component%20Object%20Reference) (OtherBodyIndex :type Integer))
  ;[1 1 1] Player go out props range
  (bind _asbp_character (Utilities|Casting|CastToBP_Character OtherActor))
  (Variables|/Game/Blueprint/Character/BP_Character.BP_Character_C|SetPropsRef _asbp_character 0)
  (Default|InteractPreview (Variables|/SettingManager/SceneManager/Blueprint/BPC_SceneManager.BPC_SceneManager_C|GetHUDWidget (Actor|GetComponentbyClass (Game|GetGameMode) "/SettingManager/SceneManager/Blueprint/BPC_SceneManager.BPC_SceneManager_C")) false))

(event EventBeginPlay
  ;[1 1 1] BeginPlay
  (CallFunction|InitValue))

(fn ConstructionScript)

(fn Interact)

(fn Action)

(fn SubAction)

(fn InitValue)