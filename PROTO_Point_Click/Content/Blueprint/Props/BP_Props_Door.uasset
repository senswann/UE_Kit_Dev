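; Door prop that opens when the player's inventory holds the required key quantity, optionally consuming it.
; InitValue loads key and objective settings from DT_Props by NameID, and Interact checks them before calling Action.
; Action reports the objective and plays an optional Level Sequence, hiding the door and disabling collision once open.
; SubAction closes it by restoring visibility and reversing the sequence, re-enabling the Box collision when playback stops.
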(event Custom|EventStopSequence
  ;[1 1 1] Event when sequence end
  (if (Variables|LevelSequence|GetIsReversePlay?)
    (Collision|SetCollisionEnabled (Variables|Default|GetBox) "QueryAndPhysics")
    (else
      (Rendering|SetActorHiddenInGame true)
      (Collision|SetCollisionEnabled (Variables|Default|GetStaticMesh) "NoCollision"))))

(event EventBeginPlay
  (|CallParentFunction)
  ;[1 1 1] Create Level Sequence player
  (bind _returnvalue (Sequencer|Player|CreateLevelSequencePlayer (Variables|LevelSequence|GetLevel%20Sequence)))
  (bind _output_get (Variables|LevelSequence|SetLevelSequencePlayer _returnvalue))
  (Utilities|IsValid _output_get
    (:Is%20Valid
      (EventDispatchers|BindEventtoOnStop _output_get (delegate Custom|EventStopSequence)))))

(fn ConstructionScript
  (|CallParentFunction))

(fn Interact
  (bind _returnvalue (Game|Player|GetPlayerPawn 0))
  (bind _keyidneed (Variables|Default|GetKeyIDNeed))
  (bind _keyquantity (Variables|Default|GetKeyQuantity))
  (bind _returnvalue_2 (Actor|GetComponentbyClass _returnvalue "/QuestSystem/Inventory/BPC_InventoryComponent.BPC_InventoryComponent_C"))
  ;[1 1 1] check if key need t oopen door
  (|CallParentFunction)
  (if (Variables|Default|GetIsKeyConsume)
    (bind _canremove_ (Default|RemovetoInvetory _returnvalue_2 _keyidneed _keyquantity))
    (if _canremove_
      (CallFunction|Action :!label _label))
    (else
      (bind _value (Default|QuerryInventory _returnvalue_2 _keyidneed))
      (if (>= _value _keyquantity)
        (goto _label)))))

(fn Action
  (bind _levelsequenceplayer (Variables|LevelSequence|GetLevelSequencePlayer))
  ;[1 1 1] Open door
  (|CallParentFunction)
  (Default|CallOnObjectiveIDCalled (CallFunction|GetMyPlayerCharacter) (Utilities|String|ToString(Name) (Variables|Default|GetObjectifID)) 1)
  (Collision|SetCollisionEnabled (Variables|Default|GetBox) "NoCollision")
  (Utilities|IsValid _levelsequenceplayer
    (:Is%20Valid
      (Variables|LevelSequence|SetIsReversePlay? false)
      (Sequencer|Player|Play _levelsequenceplayer :!class /Script/MovieScene.MovieSceneSequencePlayer))
    (:Is%20Not%20Valid
      (Rendering|SetActorHiddenInGame true)
      (Collision|SetCollisionEnabled (Variables|Default|GetStaticMesh) "NoCollision"))))

(fn SubAction
  (bind _levelsequenceplayer (Variables|LevelSequence|GetLevelSequencePlayer))
  ;[1 1 1] Close the door
  (|CallParentFunction)
  (Rendering|SetActorHiddenInGame false)
  (Collision|SetCollisionEnabled (Variables|Default|GetStaticMesh) "QueryAndPhysics")
  (Utilities|IsValid _levelsequenceplayer
    (:Is%20Valid
      (Variables|LevelSequence|SetIsReversePlay? true)
      (Class|MovieSceneSequencePlayer|PlayReverse _levelsequenceplayer))
    (:Is%20Not%20Valid
      (Collision|SetCollisionEnabled (Variables|Default|GetBox) "QueryAndPhysics"))))

(fn InitValue
  ;[1 1 1] Init Value
  (|CallParentFunction)
  (bind _returnvalue (Utilities|GetDataTableRow "/Game/GameRule/Other/Props/DT_Props.DT_Props" "Props")
    (:then
      (Variables|Default|SetKeyIDNeed (.KeyID (Utilities|Struct|BreakSTR_Props_Door (.Value (Utilities|Map|Find (.Props_Door (Utilities|Struct|BreakSTR_Props _returnvalue)) (Variables|Default|GetNameID))))))
      (Variables|Default|SetKeyQuantity (.Quantity (Utilities|Struct|BreakSTR_Props_Door (.Value (Utilities|Map|Find (.Props_Door (Utilities|Struct|BreakSTR_Props _returnvalue)) (Variables|Default|GetNameID))))))
      (Variables|Default|SetIsKeyConsume (.IsKeyCOnsume (Utilities|Struct|BreakSTR_Props_Door (.Value (Utilities|Map|Find (.Props_Door (Utilities|Struct|BreakSTR_Props _returnvalue)) (Variables|Default|GetNameID))))))
      (Variables|Default|SetObjectifID (.ObjectifID (Utilities|Struct|BreakSTR_Props_Door (.Value (Utilities|Map|Find (.Props_Door (Utilities|Struct|BreakSTR_Props _returnvalue)) (Variables|Default|GetNameID)))))))))