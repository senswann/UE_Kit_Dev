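; Player character Blueprint that hooks the quest log, dialog and prop interaction into input and game flow.
; On begin play it binds quest completion, waits a tick, loads saved quest data and checks the game mode for auto-accept quests.
; Completing any quest ends the game through the game mode's scene manager, which also handles pause.
; The interact input triggers the current dialog or referenced prop when valid.
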(event Custom|QuestComplete
  (params (QuestActor :type Object%20Object%20Reference))
  ;[0.5851 0.1701 1] Event begin play
  ;;[1 1 1] Call end when quest complete
  (Default|EndGame (Actor|GetComponentbyClass (Game|GetGameMode) "/SettingManager/SceneManager/Blueprint/BPC_SceneManager.BPC_SceneManager_C")))

(event EventBeginPlay
  ;[0.5851 0.1701 1] Event begin play
  ;;[1 1 1] Call end when quest complete
  (EventDispatchers|BindEventtoOnQuestComplete (Variables|Default|GetBPC_QuestLogComponent) (delegate Custom|QuestComplete))
  (Utilities|FlowControl|DelayUntilNextTick)
  ;;[1 1 1] Load Quests if need
  (CallFunction|LoadDataQuestSystem (Variables|Default|GetBPC_QuestLogComponent))
  ;;[1 1 1] Check If need Add Main Quest
  (Default|IsAnyQuestAutoAccept (Actor|GetComponentbyClass (Game|GetGameMode) "/QuestSystem/BPC_GM_CheckAutoAccept.BPC_GM_CheckAutoAccept_C") (Variables|Default|GetBPC_QuestLogComponent)))

(event Input|EnhancedActionEvents|EnhancedInputActionIA_Interact
  (params (ActionValue :type Boolean) (ElapsedSeconds :type Float%20%28double-precision%29) (TriggeredSeconds :type Float%20%28double-precision%29) (InputAction :type Input%20Action%20Object%20Reference :default "/Game/Input/Actions/IA_Interact.IA_Interact"))
  (bind _propsref (Variables|Default|GetPropsRef))
  ;[0.5851 0.1701 1] Interact Input
  ;;[1 1 1] Interact props input
  (Utilities|IsValid _propsref
    (:Is%20Valid
      (Default|Interact _propsref))))

(event Input|EnhancedActionEvents|EnhancedInputActionIA_Interact
  (params (ActionValue :type Boolean) (ElapsedSeconds :type Float%20%28double-precision%29) (TriggeredSeconds :type Float%20%28double-precision%29) (InputAction :type Input%20Action%20Object%20Reference :default "/Game/Input/Actions/IA_Interact.IA_Interact"))
  (bind _bpc_dialogcomponent (Variables|Default|GetBPC_DialogComponent))
  (bind _dialogref (Variables|/DialogSystem/Blueprint/BPC_DialogComponent.BPC_DialogComponent_C|GetDialogRef _bpc_dialogcomponent))
  ;[0.5851 0.1701 1] Interact Input
  ;;[1 1 1] Interact dialog input
  (Utilities|IsValid _dialogref
    (:Is%20Valid
      (Default|Interact _dialogref))))

(event Input|EnhancedActionEvents|EnhancedInputActionIA_Pause
  (params (ActionValue :type Boolean) (ElapsedSeconds :type Float%20%28double-precision%29) (TriggeredSeconds :type Float%20%28double-precision%29) (InputAction :type Input%20Action%20Object%20Reference :default "/Game/Input/Actions/IA_Pause.IA_Pause"))
  ;[1 1 1] Pause Input
  (Default|PauseMenu (Actor|GetComponentbyClass (Game|GetGameMode) "/SettingManager/SceneManager/Blueprint/BPC_SceneManager.BPC_SceneManager_C")))

(fn ConstructionScript)