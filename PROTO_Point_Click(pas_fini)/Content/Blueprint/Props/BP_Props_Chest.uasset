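; Chest prop that the player opens with key items from their inventory to receive item rewards.
; InitValue loads key, quantity, consume flag, rewards and objective ID from DT_Props by NameID.
; Interact either removes the keys or only checks the held count, then calls Action.
; Action adds the rewards through BPC_InventoryComponent, disables the Box collision and reports the objective ID to the player character.
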(event EventBeginPlay
  (|CallParentFunction))

(event Collision|EventActorBeginOverlap
  (params (OtherActor :type Actor%20Object%20Reference)))

(event EventTick
  (params (DeltaSeconds :type Float%20%28single-precision%29)))

(fn ConstructionScript
  (|CallParentFunction))

(fn Interact
  (bind _returnvalue (Game|Player|GetPlayerPawn 0))
  (bind _keyid (Variables|Default|GetKeyID))
  (bind _quantity (Variables|Default|GetQuantity))
  (bind _returnvalue_2 (Actor|GetComponentbyClass _returnvalue "/QuestSystem/Inventory/BPC_InventoryComponent.BPC_InventoryComponent_C"))
  ;[1 1 1] Check to Open chest
  (|CallParentFunction)
  (if (Variables|Default|GetIsKeyConsume)
    (bind _canremove_ (Default|RemovetoInvetory _returnvalue_2 _keyid _quantity))
    (if _canremove_
      (CallFunction|Action :!label _label))
    (else
      (bind _value (Default|QuerryInventory _returnvalue_2 _keyid))
      (if (>= _value _quantity)
        (goto _label)))))

(fn Action
  (bind _itemsreward (Variables|Default|GetItemsReward))
  ;[1 1 1] OpenChest and add reward to player
  (|CallParentFunction)
  (LocalVariables|SetPlayerInventory (Actor|GetComponentbyClass (Game|Player|GetPlayerPawn 0) "/QuestSystem/Inventory/BPC_InventoryComponent.BPC_InventoryComponent_C"))
  (bind _values (Utilities|Map|Values _itemsreward))
  (bind _keys (Utilities|Map|Keys _itemsreward))
  (for (_array_element _array_index) _keys
    (Default|AddtoInventory (LocalVariables|GetPlayerInventory) _array_element (Utilities|Array|Get(acopy) _values _array_index)))
  (Collision|SetCollisionEnabled (Variables|Default|GetBox) "NoCollision")
  (Default|CallOnObjectiveIDCalled (CallFunction|GetMyPlayerCharacter) (Utilities|String|ToString(Name) (Variables|Default|GetObjectifID)) 1))

(fn InitValue
  ;[1 1 1] Init Value
  (|CallParentFunction)
  (bind _returnvalue (Utilities|GetDataTableRow "/Game/GameRule/Other/Props/DT_Props.DT_Props" "Props")
    (:then
      (Variables|Default|SetKeyID (.KeyID (Utilities|Struct|BreakSTR_Props_Chest (.Value (Utilities|Map|Find (.Props_Chest (Utilities|Struct|BreakSTR_Props _returnvalue)) (Variables|Default|GetNameID))))))
      (Variables|Default|SetIsKeyConsume (.IsKeyConsume (Utilities|Struct|BreakSTR_Props_Chest (.Value (Utilities|Map|Find (.Props_Chest (Utilities|Struct|BreakSTR_Props _returnvalue)) (Variables|Default|GetNameID))))))
      (Variables|Default|SetQuantity (.Quantity (Utilities|Struct|BreakSTR_Props_Chest (.Value (Utilities|Map|Find (.Props_Chest (Utilities|Struct|BreakSTR_Props _returnvalue)) (Variables|Default|GetNameID))))))
      (Variables|Default|SetItemsReward (.Item_Reward (Utilities|Struct|BreakSTR_Props_Chest (.Value (Utilities|Map|Find (.Props_Chest (Utilities|Struct|BreakSTR_Props _returnvalue)) (Variables|Default|GetNameID))))))
      (Variables|Default|SetObjectifID (.ObjectifID (Utilities|Struct|BreakSTR_Props_Chest (.Value (Utilities|Map|Find (.Props_Chest (Utilities|Struct|BreakSTR_Props _returnvalue)) (Variables|Default|GetNameID)))))))))