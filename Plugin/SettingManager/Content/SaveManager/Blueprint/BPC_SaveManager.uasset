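; Save manager component that persists the player's transform and audio volume settings in a single BP_SaveData slot.
; On BeginPlay it loads and applies both, or creates the slot with the current player transform.
; Separate player and sound events save to the slot or reapply from the cached object, only while the slot exists, with volumes routed through the GameMode's BPC_AudioManager.
; It also deletes the slot and opens a paused save-settings widget.
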(event EventBeginPlay
  (bind _returnvalue (SaveGame|DoesSaveGameExist "SaveData"))
  (if _returnvalue
    ;[1 1 1] If exist, load data
    (bind _returnvalue_2 (SaveGame|LoadGamefromSlot "SaveData"))
    (bind _asbp_save_data (Utilities|Casting|CastToBP_SaveData _returnvalue_2))
    (Variables|Default|SetSaveData _asbp_save_data)
    (CallFunction|LoadDataPlayer (Default|GetPlayerData (Variables|Default|GetSaveData)))
    (CallFunction|LoadDataSound (Default|GetSoundData (Variables|Default|GetSaveData)))
    (else
      ;[1 1 1] If no save exist, create one
      (bind _returnvalue_3 (SaveGame|CreateSaveGameObject "/SettingManager/SaveManager/Blueprint/BP_SaveData.BP_SaveData_C"))
      (bind _output_get (Variables|Default|SetSaveData _returnvalue_3))
      (CallFunction|GetDataPlayer)
      (SaveGame|SaveGametoSlot _output_get "SaveData"))))

(fn GetDataPlayer
  ;[1 1 1] Get data from player
  (Default|SetDataPlayerValue (Variables|Default|GetSaveData) (Transformation|GetActorTransform (Game|Player|GetPlayerPawn 0))))

(fn GetDataSound
  ;[1 1 1] Get sound Data
  (Default|SetDataSoundValue (Variables|Default|GetSaveData) (Variables|/SettingManager/AudioManager/Blueprint/BPC_AudioManager.BPC_AudioManager_C|GetSoundMap (Actor|GetComponentbyClass (Game|GetGameMode) "/SettingManager/AudioManager/Blueprint/BPC_AudioManager.BPC_AudioManager_C"))))

(fn LoadDataPlayer
  (params (NewTransform :type Transform%20%28by%20ref%29))
  ;[1 1 1] Set data to player
  (Transformation|SetActorTransform (Game|Player|GetPlayerPawn 0) NewTransform false true))

(fn LoadDataSound
  (params (SoundMap :type Map%20of%20Sound%20Class%20Object%20References%20to%20Reals))
  ;[1 1 1] Set audio manager value
  (bind _keys (Utilities|Map|Keys SoundMap))
  (for _array_element _keys
    (Default|UpdateSound (Actor|GetComponentbyClass (Game|GetGameMode) "/SettingManager/AudioManager/Blueprint/BPC_AudioManager.BPC_AudioManager_C") (.Value (Utilities|Map|Find SoundMap _array_element)) _array_element)))

(fn PlayerSaveEvent
  ;[1 1 1] Save sytem Logic
  (bind _returnvalue (SaveGame|DoesSaveGameExist "SaveData"))
  (if _returnvalue
    (CallFunction|GetDataPlayer)
    (SaveGame|SaveGametoSlot (Variables|Default|GetSaveData) "SaveData")))

(fn SoundSaveEvent
  ;[1 1 1] SavceAudio
  (bind _returnvalue (SaveGame|DoesSaveGameExist "SaveData"))
  (if _returnvalue
    (CallFunction|GetDataSound)
    (SaveGame|SaveGametoSlot (Variables|Default|GetSaveData) "SaveData")))

(fn PlayerLoadEvent
  ;[1 1 1] Load system logic
  (bind _returnvalue (SaveGame|DoesSaveGameExist "SaveData"))
  (if _returnvalue
    (CallFunction|LoadDataPlayer (Default|GetPlayerData (Variables|Default|GetSaveData)))))

(fn SoundLoadEvent
  ;[1 1 1] Load sound
  (bind _returnvalue (SaveGame|DoesSaveGameExist "SaveData"))
  (if _returnvalue
    (CallFunction|LoadDataSound (Variables|/SettingManager/SaveManager/Blueprint/BP_SaveData.BP_SaveData_C|GetSound_volume (Variables|Default|GetSaveData)))))

(fn DeleteEvent
  ;[1 1 1] Delete save
  (SaveGame|DeleteGameinSlot "SaveData"))

(fn LoadSaveSetting
  (bind _returnvalue (Game|GetPlayerController 0))
  ;[1 1 1] Load save setting widget
  (Viewport|RemoveAllWidgets)
  (bind _returnvalue_2 (UserInterface|CreateWidget (Variables|Default|GetWBP_SaveSetting)))
  (UserInterface|Viewport|AddtoViewport _returnvalue_2 0)
  (Game|SetGamePaused true)
  (Variables|/Script/Engine.PlayerController|SetbShowMouseCursor _returnvalue true)
  (Input|SetInputModeUIOnly _returnvalue _returnvalue_2 "DoNotLock" false))