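; BPC_AudioManager is an audio manager Blueprint that applies volume changes and opens the audio settings menu.
; UpdateSound overrides a given sound class's volume on the SCM_MasterVolume mix, then pushes that mix.
; LoadAudioSetting clears all widgets, shows WBPAudioSetting, pauses the game and switches player 0 to UI-only input with a visible cursor.
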(event EventBeginPlay)

(event EventTick
  (params (DeltaSeconds :type Float%20%28single-precision%29)))

(fn UpdateSound
  (params (Volume :type Float%20%28double-precision%29) (SoundClass :type Sound%20Class%20Object%20Reference))
  ;[1 1 1] UpdateSound
  (Audio|SetSoundMixClassOverride "/SettingManager/AudioManager/Sound/SCM_MasterVolume.SCM_MasterVolume" SoundClass Volume 1.0 1.0 true)
  (Audio|PushSoundMixModifier "/SettingManager/AudioManager/Sound/SCM_MasterVolume.SCM_MasterVolume"))

(fn LoadAudioSetting
  (bind _returnvalue (Game|GetPlayerController 0))
  ;[1 1 1] Remove all widget & pause game & Add Widget
  (Viewport|RemoveAllWidgets)
  (bind _returnvalue_2 (UserInterface|CreateWidget (Variables|Default|GetWBPAudioSetting)))
  (UserInterface|Viewport|AddtoViewport _returnvalue_2 0)
  (Game|SetGamePaused true)
  (Variables|/Script/Engine.PlayerController|SetbShowMouseCursor _returnvalue true)
  (Input|SetInputModeUIOnly _returnvalue _returnvalue_2 "DoNotLock" false))