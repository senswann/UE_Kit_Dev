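; Health component that tracks player health, damage, healing and death, and drives an optional health widget.
; SetUpHealthSystem stores the widget, display flags and invincibility delay, then fills health to maximum.
; Healing and damage clamp health and refresh the widget, with damage starting a timed invincibility window and calling CallDeathOfPlayer at zero.
; The health text updates only when the health bar is also active.
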(event Custom|Inviciblity
  ;[1 1 1] Invicible Event
  (Variables|Default|SetIsInvicible true)
  (Utilities|FlowControl|Delay (Variables|Default|GetInvicibilityDelay))
  (Variables|Default|SetIsInvicible false))

(fn SetHealth
  (params (MaxHeatlh :type Integer))
  ;[1 1 1] Init value
  (Variables|Default|SetCurrentHealth MaxHeatlh)
  (Variables|Default|SetMaxHealth MaxHeatlh)
  (CallFunction|UpdateWBPHealth))

(fn IncreaseHealth
  (params (IncreaseHealthValue :type Integer))
  ;[1 1 1] Increase Health of the player
  (if (> (+ (Variables|Default|GetCurrentHealth) IncreaseHealthValue) (Variables|Default|GetMaxHealth))
    (Variables|Default|SetCurrentHealth (Variables|Default|GetMaxHealth))
    (else
      (Variables|Default|SetCurrentHealth (+ (Variables|Default|GetCurrentHealth) IncreaseHealthValue))))
  (CallFunction|UpdateWBPHealth))

(fn DecreaseHealth
  (params (DecreaseHealthValue :type Integer))
  ;[1 1 1] Decrease health & call death if 0 hp
  (if (not (Variables|Default|GetIsInvicible))
    (CallFunction|Inviciblity)
    (if (<= (- (Variables|Default|GetCurrentHealth) DecreaseHealthValue) 0)
      (Variables|Default|SetCurrentHealth 0)
      (CallFunction|UpdateWBPHealth)
      (Default|CallDeathOfPlayer)
      (else
        (Variables|Default|SetCurrentHealth (- (Variables|Default|GetCurrentHealth) DecreaseHealthValue))
        (CallFunction|UpdateWBPHealth)))))

(fn UpdateWBPHealth
  (bind _currenthealth (Variables|Default|GetCurrentHealth))
  (bind _maxhealth (Variables|Default|GetMaxHealth))
  ;[1 1 1] Update HealthBar or Health if need
  (bind _wbphealth (Variables|Default|GetWBPHealth)
    (:then
      (if (Variables|Default|GetIsHeatlhBarActive)
        (Default|UpdateHealthBar _wbphealth _currenthealth _maxhealth)
        (if (Variables|Default|GetIsHealthTextActive)
          (Default|UpdateHealth _wbphealth _currenthealth _maxhealth))))
    (:else)))

(fn SetUpHealthSystem
  (params (MaxHealth :type Integer) (HealthWidget :type WBP%20Health%20Object%20Reference) (IsHealthTextActive :type Boolean) (IsHealthBarActive :type Boolean) (InvicibilityDelay :type Float%20%28double-precision%29))
  ;[0.4331 0.1058 1] Set up of health system value
  ;;[1 1 1] Set Widget
  (Utilities|IsValid HealthWidget
    (:Is%20Valid
      (Variables|Default|SetWBPHealth HealthWidget))
    (:Is%20Not%20Valid
      _))
  ;;[1 1 1] Set if what need to be update in the widget
  (Variables|Default|SetIsHealthTextActive IsHealthTextActive)
  (Variables|Default|SetIsHeatlhBarActive IsHealthBarActive)
  ;;[1 1 1] invicibility time
  (Variables|Default|SetInvicibilityDelay InvicibilityDelay)
  ;;[1 1 1] Set hp
  (CallFunction|SetHealth MaxHealth))